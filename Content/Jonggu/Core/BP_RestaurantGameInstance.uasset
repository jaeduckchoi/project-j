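; Game instance for a restaurant prototype that holds session state (day, clams, revenue, menu, guests, service summary) and persists it as checkpoints.
; On Init it loads or creates a BP_PrototypeSave slot, copying fields both ways with a schema version check on load.
; CollectClam uses a bitmask to allow one harvest per point; BeginNextDay resets daily state from phase 2 and saves.
; Every step feeds a numbered debug event log with a state snapshot.
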(event EventInit
  (CallFunction|InitializeSession))

(fn InitializeSession
  (if (not (Variables|Default|Getinitialized))
    (Variables|Default|Setinitialized true)
    (bind _returnvalue (SaveGame|DoesSaveGameExist (Variables|Default|Getsave_slot)))
    (if _returnvalue
      (CallFunction|LoadCheckpoint)
      (else
        (CallFunction|SaveCheckpoint)))
    (CallFunction|LogEvent "session_initialized"))
  (return))

(fn SaveCheckpoint
  (Variables|Default|Setsave_ok false)
  (bind _returnvalue (SaveGame|CreateSaveGameObject "/Game/Jonggu/Core/Save/BP_PrototypeSave.BP_PrototypeSave_C"))
  (bind _asbp_prototype_save (Utilities|Casting|CastToBP_PrototypeSave _returnvalue)
    (:then
      _)
    (:CastFailed
      _))
  (if (Utilities|IsValid _asbp_prototype_save)
    (Variables|/Game/Jonggu/Core/Save/BP_PrototypeSave.BP_PrototypeSave_C|Setschema_version _asbp_prototype_save 1)
    (Variables|/Game/Jonggu/Core/Save/BP_PrototypeSave.BP_PrototypeSave_C|Setday _asbp_prototype_save (Variables|Default|Getday))
    (Variables|/Game/Jonggu/Core/Save/BP_PrototypeSave.BP_PrototypeSave_C|Setclams _asbp_prototype_save (Variables|Default|Getclams))
    (Variables|/Game/Jonggu/Core/Save/BP_PrototypeSave.BP_PrototypeSave_C|Setharvested_mask _asbp_prototype_save (Variables|Default|Getharvested_mask))
    (Variables|/Game/Jonggu/Core/Save/BP_PrototypeSave.BP_PrototypeSave_C|Setmenu_mask _asbp_prototype_save (Variables|Default|Getmenu_mask))
    (Variables|/Game/Jonggu/Core/Save/BP_PrototypeSave.BP_PrototypeSave_C|Setguest_target _asbp_prototype_save (Variables|Default|Getguest_target))
    (Variables|/Game/Jonggu/Core/Save/BP_PrototypeSave.BP_PrototypeSave_C|Settotal_revenue _asbp_prototype_save (Variables|Default|Gettotal_revenue))
    (Variables|/Game/Jonggu/Core/Save/BP_PrototypeSave.BP_PrototypeSave_C|Setcheckpoint_phase _asbp_prototype_save (Variables|Default|Getcheckpoint_phase))
    (Variables|/Game/Jonggu/Core/Save/BP_PrototypeSave.BP_PrototypeSave_C|Setcheckpoint_map _asbp_prototype_save (Variables|Default|Getcheckpoint_map))
    (Variables|/Game/Jonggu/Core/Save/BP_PrototypeSave.BP_PrototypeSave_C|Setentry_marker _asbp_prototype_save (Variables|Default|Getentry_marker))
    (Variables|/Game/Jonggu/Core/Save/BP_PrototypeSave.BP_PrototypeSave_C|Setsummary_served _asbp_prototype_save (Variables|Default|Getsummary_served))
    (Variables|/Game/Jonggu/Core/Save/BP_PrototypeSave.BP_PrototypeSave_C|Setsummary_base _asbp_prototype_save (Variables|Default|Getsummary_base))
    (Variables|/Game/Jonggu/Core/Save/BP_PrototypeSave.BP_PrototypeSave_C|Setsummary_bonus _asbp_prototype_save (Variables|Default|Getsummary_bonus))
    (Variables|/Game/Jonggu/Core/Save/BP_PrototypeSave.BP_PrototypeSave_C|Setsummary_clams_used _asbp_prototype_save (Variables|Default|Getsummary_clams_used))
    (Variables|/Game/Jonggu/Core/Save/BP_PrototypeSave.BP_PrototypeSave_C|Setsummary_special_served _asbp_prototype_save (Variables|Default|Getsummary_special_served))
    (bind _returnvalue_2 (SaveGame|SaveGametoSlot _asbp_prototype_save (Variables|Default|Getsave_slot)))
    (Variables|Default|Setsave_ok _returnvalue_2))
  (if (Variables|Default|Getsave_ok)
    (CallFunction|LogEvent "checkpoint_saved")
    (else
      (CallFunction|LogEvent "checkpoint_save_failed")
      (Development|PrintString "저장하지 못했습니다. 현재 플레이는 유지됩니다." true true "(R=0.000000,G=0.660000,B=1.000000,A=1.000000)" 8.0)))
  (return (Variables|Default|Getsave_ok)))

(fn LoadCheckpoint
  (Variables|Default|Setsave_ok false)
  (bind _returnvalue (SaveGame|LoadGamefromSlot (Variables|Default|Getsave_slot)))
  (bind _asbp_prototype_save (Utilities|Casting|CastToBP_PrototypeSave _returnvalue)
    (:then
      _)
    (:CastFailed
      _))
  (if (Utilities|IsValid _asbp_prototype_save)
    (if (== (Variables|/Game/Jonggu/Core/Save/BP_PrototypeSave.BP_PrototypeSave_C|Getschema_version _asbp_prototype_save) 1)
      (Variables|Default|Setday (Variables|/Game/Jonggu/Core/Save/BP_PrototypeSave.BP_PrototypeSave_C|Getday _asbp_prototype_save))
      (Variables|Default|Setclams (Variables|/Game/Jonggu/Core/Save/BP_PrototypeSave.BP_PrototypeSave_C|Getclams _asbp_prototype_save))
      (Variables|Default|Setharvested_mask (Variables|/Game/Jonggu/Core/Save/BP_PrototypeSave.BP_PrototypeSave_C|Getharvested_mask _asbp_prototype_save))
      (Variables|Default|Setmenu_mask (Variables|/Game/Jonggu/Core/Save/BP_PrototypeSave.BP_PrototypeSave_C|Getmenu_mask _asbp_prototype_save))
      (Variables|Default|Setguest_target (Variables|/Game/Jonggu/Core/Save/BP_PrototypeSave.BP_PrototypeSave_C|Getguest_target _asbp_prototype_save))
      (Variables|Default|Settotal_revenue (Variables|/Game/Jonggu/Core/Save/BP_PrototypeSave.BP_PrototypeSave_C|Gettotal_revenue _asbp_prototype_save))
      (Variables|Default|Setcheckpoint_phase (Variables|/Game/Jonggu/Core/Save/BP_PrototypeSave.BP_PrototypeSave_C|Getcheckpoint_phase _asbp_prototype_save))
      (Variables|Default|Setcheckpoint_map (Variables|/Game/Jonggu/Core/Save/BP_PrototypeSave.BP_PrototypeSave_C|Getcheckpoint_map _asbp_prototype_save))
      (Variables|Default|Setentry_marker (Variables|/Game/Jonggu/Core/Save/BP_PrototypeSave.BP_PrototypeSave_C|Getentry_marker _asbp_prototype_save))
      (Variables|Default|Setsummary_served (Variables|/Game/Jonggu/Core/Save/BP_PrototypeSave.BP_PrototypeSave_C|Getsummary_served _asbp_prototype_save))
      (Variables|Default|Setsummary_base (Variables|/Game/Jonggu/Core/Save/BP_PrototypeSave.BP_PrototypeSave_C|Getsummary_base _asbp_prototype_save))
      (Variables|Default|Setsummary_bonus (Variables|/Game/Jonggu/Core/Save/BP_PrototypeSave.BP_PrototypeSave_C|Getsummary_bonus _asbp_prototype_save))
      (Variables|Default|Setsummary_clams_used (Variables|/Game/Jonggu/Core/Save/BP_PrototypeSave.BP_PrototypeSave_C|Getsummary_clams_used _asbp_prototype_save))
      (Variables|Default|Setsummary_special_served (Variables|/Game/Jonggu/Core/Save/BP_PrototypeSave.BP_PrototypeSave_C|Getsummary_special_served _asbp_prototype_save))
      (Variables|Default|Setsave_ok true)))
  (if (Variables|Default|Getsave_ok)
    (CallFunction|LogEvent "checkpoint_loaded")
    (else
      (CallFunction|LogEvent "checkpoint_load_failed_state_preserved")
      (Development|PrintString "저장을 불러오지 못했습니다. 현재 상태를 유지합니다." true true "(R=0.000000,G=0.660000,B=1.000000,A=1.000000)" 8.0)))
  (return (Variables|Default|Getsave_ok)))

(fn CollectClam
  (params (point_bit :type Integer))
  (if (and (or (or (== point_bit 1) (== point_bit 2)) (== point_bit 4)) (== (Class|KismetMathLibrary|AndIntInt (Variables|Default|Getharvested_mask) point_bit) 0))
    (Variables|Default|Setharvested_mask (Class|KismetMathLibrary|OrIntInt (Variables|Default|Getharvested_mask) point_bit))
    (Variables|Default|Setclams (+ (Variables|Default|Getclams) 1))
    (CallFunction|LogEvent (Utilities|String|Append "clam_collected point=" (Utilities|String|ToString(Integer) point_bit)))
    (return true)
    (else
      (return false))))

(fn BeginNextDay
  (if (== (Variables|Default|Getcheckpoint_phase) 2)
    (Variables|Default|Setcheckpoint_phase 0)
    (Variables|Default|Setday (+ (Variables|Default|Getday) 1))
    (Variables|Default|Setharvested_mask 0)
    (Variables|Default|Setcheckpoint_map "L_Hub")
    (Variables|Default|Setentry_marker "HubArrival")
    (Variables|Default|Setsummary_served 0)
    (Variables|Default|Setsummary_base 0)
    (Variables|Default|Setsummary_bonus 0)
    (Variables|Default|Setsummary_clams_used 0)
    (Variables|Default|Setsummary_special_served 0)
    (CallFunction|LogEvent "next_day_preparation")
    (CallFunction|SaveCheckpoint))
  (return))

(fn LogEvent
  (params (event_text :type String))
  (Variables|Default|Setevent_count (+ (Variables|Default|Getevent_count) 1))
  (Variables|Default|Setevent_log (Utilities|String|Append (Utilities|String|Append (Variables|Default|Getevent_log) (Utilities|String|Append (Utilities|String|Append (Utilities|String|Append (Utilities|String|Append (Utilities|String|Append (Utilities|String|Append (Utilities|String|Append (Utilities|String|Append (Utilities|String|Append (Utilities|String|Append (Utilities|String|Append (Utilities|String|Append (Utilities|String|Append "[JongguPrototype] #" (Utilities|String|ToString(Integer) (Variables|Default|Getevent_count))) " day=") (Utilities|String|ToString(Integer) (Variables|Default|Getday))) " clams=") (Utilities|String|ToString(Integer) (Variables|Default|Getclams))) " revenue=") (Utilities|String|ToString(Integer) (Variables|Default|Gettotal_revenue))) " menu_mask=") (Utilities|String|ToString(Integer) (Variables|Default|Getmenu_mask))) " guests=") (Utilities|String|ToString(Integer) (Variables|Default|Getguest_target))) " event=") event_text)) "
"))
  (Development|PrintString (Utilities|String|Append (Utilities|String|Append (Utilities|String|Append (Utilities|String|Append (Utilities|String|Append (Utilities|String|Append (Utilities|String|Append (Utilities|String|Append (Utilities|String|Append (Utilities|String|Append (Utilities|String|Append (Utilities|String|Append (Utilities|String|Append "[JongguPrototype] #" (Utilities|String|ToString(Integer) (Variables|Default|Getevent_count))) " day=") (Utilities|String|ToString(Integer) (Variables|Default|Getday))) " clams=") (Utilities|String|ToString(Integer) (Variables|Default|Getclams))) " revenue=") (Utilities|String|ToString(Integer) (Variables|Default|Gettotal_revenue))) " menu_mask=") (Utilities|String|ToString(Integer) (Variables|Default|Getmenu_mask))) " guests=") (Utilities|String|ToString(Integer) (Variables|Default|Getguest_target))) " event=") event_text) false)
  (return))