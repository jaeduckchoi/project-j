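; Player pawn for a 2D sprite character that moves on the X-Z plane with polled WASD or arrow keys.
; Each locally controlled tick updates four-way facing, with bias against diagonal flicker and mirrored side sprites.
; Idle plays two-frame sprites; walking swaps in separate head, body and foot sprites, offset procedurally from a distance-driven eight-step phase.
; The visual also bobs and leans, and translucent sort priority follows world Z for depth ordering.
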(event EventTick
  (params (DeltaSeconds :type Float%20%28single-precision%29))
  (bind _returnvalue (Game|GetPlayerController 0))
  (if (Pawn|IsLocallyControlled)
    (Variables|/Script/Engine.FloatingPawnMovement|SetMaxSpeed (Variables|Default|Getmovement_component) (Math|Float|Max(Float) (Variables|Player|Getmove_speed) 0.0))
    (Pawn|Input|AddMovementInput (Math|Vector|Normalize (Math|Vector|MakeVector (- (Math|Float|Max(Float) (Class|PlayerController|GetInputAnalogKeyState _returnvalue "D") (Class|PlayerController|GetInputAnalogKeyState _returnvalue "Right")) (Math|Float|Max(Float) (Class|PlayerController|GetInputAnalogKeyState _returnvalue "A") (Class|PlayerController|GetInputAnalogKeyState _returnvalue "Left"))) 0.0 (- (Math|Float|Max(Float) (Class|PlayerController|GetInputAnalogKeyState _returnvalue "W") (Class|PlayerController|GetInputAnalogKeyState _returnvalue "Up")) (Math|Float|Max(Float) (Class|PlayerController|GetInputAnalogKeyState _returnvalue "S") (Class|PlayerController|GetInputAnalogKeyState _returnvalue "Down"))))) 1.0 false)
    (CallFunction|RefreshPlayerVisual)))

(event EventBeginPlay
  (bind _returnvalue (Transformation|GetActorLocation))
  (Components|Movement|SetUpdatedComponent (Variables|Default|Getmovement_component) (Variables|Default|Getcollision_component))
  (Class|MovementComponent|SetPlaneConstraintOrigin (Variables|Default|Getmovement_component) _returnvalue)
  (Variables|Player|Motionstate|Setprevious_position _returnvalue)
  (Variables|Player|Motionstate|Setvisual_origin (Variables|/Script/Engine.SceneComponent|GetRelativeLocation (Variables|Default|Getplayer_visual)))
  (CallFunction|RefreshPlayerVisual))

(fn ConstructionScript)

(fn RefreshPlayerVisual
  (bind _returnvalue (Transformation|GetVelocity))
  (bind _returnvalue_2 (Utilities|Time|GetWorldDeltaSeconds))
  (bind _returnvalue_3 (Transformation|GetActorLocation))
  (bind _returnvalue_4 (Class|Pawn|GetPendingMovementInputVector))
  (bind _returnvalue_5 (Class|Pawn|GetLastMovementInputVector))
  (bind _player_visual (Variables|Default|Getplayer_visual))
  (bind _visual_scale (Variables|Player|Getvisual_scale))
  (bind _walk_right_foot (Variables|Default|Getwalk_right_foot))
  (bind _walk_left_foot (Variables|Default|Getwalk_left_foot))
  (bind _walk_body (Variables|Default|Getwalk_body))
  (bind _walk_head (Variables|Default|Getwalk_head))
  (bind _returnvalue_6 (Math|Vector|VectorLengthSquared _returnvalue))
  (bind (_x _y _z) (Math|Vector|BreakVector _visual_scale))
  (bind _z_2 (Math|Vector|BreakVector _returnvalue_3))
  (bind _returnvalue_7 (Math|Vector|VectorLengthSquared _returnvalue_4))
  (bind _spritecolor (Variables|/Script/Paper2D.PaperSpriteComponent|GetSpriteColor _player_visual))
  (bind _returnvalue_8 (+ _z_2 0.5))
  (bind _returnvalue_9 (> _returnvalue_7 0.0001))
  (bind _returnvalue_10 (> _returnvalue_6 1.0))
  (bind _returnvalue_11 (Math|Float|Floor _returnvalue_8))
  (bind _returnvalue_12 (Math|Vector|SelectVector _returnvalue_4 _returnvalue_5 _returnvalue_9))
  (bind (_x_2 _y_2 _z_3) (Math|Vector|BreakVector _returnvalue_12))
  (bind _returnvalue_13 (- 0 _returnvalue_11))
  (bind _returnvalue_14 (Math|Float|Absolute(Float) _x_2))
  (bind _returnvalue_15 (Math|Float|Absolute(Float) _z_3))
  (bind _returnvalue_16 (> _z_3 0.0))
  (bind _returnvalue_17 (Math|Integer|SelectInt 1 0 _returnvalue_16))
  (Variables|Player|Motionstate|Setwalk_phase (Math|Float|SelectFloat 0.0 (Math|Float|Fraction (+ (Variables|Player|Motionstate|Getwalk_phase) (/ (Math|Float|SelectFloat 0.0 (Math|Vector|VectorLength (- _returnvalue_3 (Variables|Player|Motionstate|Getprevious_position))) (> (Math|Vector|VectorLength (- _returnvalue_3 (Variables|Player|Motionstate|Getprevious_position))) (Math|Float|Max(Float) 2e+01 (* (Variables|Player|Getmove_speed) (* _returnvalue_2 4.0))))) (Math|Float|Max(Float) (Variables|Player|Getwalk_cycle_distance) 1.0)))) (and _returnvalue_10 (not (Variables|Player|Motionstate|Getis_moving)))))
  (Variables|Player|Motionstate|Setprevious_position _returnvalue_3)
  (Variables|Player|Motionstate|Setis_moving _returnvalue_10)
  (Variables|Player|Motionstate|Setfacing_direction (Math|Integer|SelectInt (Math|Integer|SelectInt (Math|Integer|SelectInt 3 2 (> _x_2 0.0)) _returnvalue_17 (or (> _returnvalue_14 (* _returnvalue_15 1.15)) (and (not (> _returnvalue_15 (* _returnvalue_14 1.15))) (not (== (Variables|Player|Motionstate|Getfacing_direction) _returnvalue_17))))) (Variables|Player|Motionstate|Getfacing_direction) (> (Math|Vector|VectorLengthSquared _returnvalue_12) 0.0001)))
  (Variables|Player|Motionstate|Setidle_elapsed (Math|Float|SelectFloat 0.0 (+ (Variables|Player|Motionstate|Getidle_elapsed) _returnvalue_2) _returnvalue_10))
  (Variables|Player|Motionstate|Setwalk_blend (Math|Interpolation|FInterpTo (Variables|Player|Motionstate|Getwalk_blend) (Math|Float|SelectFloat 1.0 0.0 _returnvalue_10) _returnvalue_2 18.0))
  (Variables|Player|Motionstate|Setcurrent_frame_index (Math|Integer|SelectInt (Math|Integer|Clamp(Integer) (Math|Float|Floor (* (Variables|Player|Motionstate|Getwalk_phase) 8.0)) 0 7) (Math|Integer|%(Integer) (Math|Float|Floor (* (Variables|Player|Motionstate|Getidle_elapsed) (Math|Float|Max(Float) (Variables|Player|Getidle_frames_per_second) 0.01))) 2) (Variables|Player|Motionstate|Getis_moving)))
  (if (>= (Variables|Player|Motionstate|Getfacing_direction) 2)
    (Rendering|Components|Sprite|SetSprite _player_visual (Utilities|Array|Get(acopy) (Variables|Player|Getside_frames) (Math|Integer|SelectInt 0 (Variables|Player|Motionstate|Getcurrent_frame_index) (Variables|Player|Motionstate|Getis_moving))))
    (Rendering|Components|Sprite|SetSprite (Variables|Default|Getwalk_head) (Utilities|Array|Get(acopy) (Variables|Player|Getside_walk_parts)))
    (Rendering|Components|Sprite|SetSprite (Variables|Default|Getwalk_body) (Utilities|Array|Get(acopy) (Variables|Player|Getside_walk_parts) 1))
    (Rendering|Components|Sprite|SetSprite (Variables|Default|Getwalk_left_foot) (Utilities|Array|Get(acopy) (Variables|Player|Getside_walk_parts) 2))
    (Rendering|Components|Sprite|SetSprite (Variables|Default|Getwalk_right_foot) (Utilities|Array|Get(acopy) (Variables|Player|Getside_walk_parts) 3))
    (elif (== (Variables|Player|Motionstate|Getfacing_direction) 1)
      (Rendering|Components|Sprite|SetSprite _player_visual (Utilities|Array|Get(acopy) (Variables|Player|Getback_frames) (Math|Integer|SelectInt 0 (Variables|Player|Motionstate|Getcurrent_frame_index) (Variables|Player|Motionstate|Getis_moving))))
      (Rendering|Components|Sprite|SetSprite (Variables|Default|Getwalk_head) (Utilities|Array|Get(acopy) (Variables|Player|Getback_walk_parts)))
      (Rendering|Components|Sprite|SetSprite (Variables|Default|Getwalk_body) (Utilities|Array|Get(acopy) (Variables|Player|Getback_walk_parts) 1))
      (Rendering|Components|Sprite|SetSprite (Variables|Default|Getwalk_left_foot) (Utilities|Array|Get(acopy) (Variables|Player|Getback_walk_parts) 2))
      (Rendering|Components|Sprite|SetSprite (Variables|Default|Getwalk_right_foot) (Utilities|Array|Get(acopy) (Variables|Player|Getback_walk_parts) 3))
      (else
        (Rendering|Components|Sprite|SetSprite _player_visual (Utilities|Array|Get(acopy) (Variables|Player|Getfront_frames) (Math|Integer|SelectInt 0 (Variables|Player|Motionstate|Getcurrent_frame_index) (Variables|Player|Motionstate|Getis_moving))))
        (Rendering|Components|Sprite|SetSprite (Variables|Default|Getwalk_head) (Utilities|Array|Get(acopy) (Variables|Player|Getfront_walk_parts)))
        (Rendering|Components|Sprite|SetSprite (Variables|Default|Getwalk_body) (Utilities|Array|Get(acopy) (Variables|Player|Getfront_walk_parts) 1))
        (Rendering|Components|Sprite|SetSprite (Variables|Default|Getwalk_left_foot) (Utilities|Array|Get(acopy) (Variables|Player|Getfront_walk_parts) 2))
        (Rendering|Components|Sprite|SetSprite (Variables|Default|Getwalk_right_foot) (Utilities|Array|Get(acopy) (Variables|Player|Getfront_walk_parts) 3)))))
  (if (Variables|Player|Motionstate|Getis_moving)
    (Rendering|Components|Sprite|SetSprite _player_visual 0))
  (Transformation|SetRelativeScale3D _player_visual (Math|Vector|MakeVector (* (Math|Float|Absolute(Float) _x) (Math|Float|SelectFloat -1.0 1.0 (or (and (== (Variables|Player|Motionstate|Getfacing_direction) 3) (Variables|Player|Getside_sprite_faces_left)) (and (== (Variables|Player|Motionstate|Getfacing_direction) 2) (not (Variables|Player|Getside_sprite_faces_left)))))) _y _z))
  (Transformation|SetRelativeLocation _player_visual (+ (Variables|Player|Motionstate|Getvisual_origin) (Math|Vector|MakeVector 0.0 0.0 (* (* (Math|Trig|Sin(Radians) (* (Variables|Player|Motionstate|Getwalk_phase) 12.566370614359172)) (Variables|Player|Getwalk_bob_cm)) (Variables|Player|Motionstate|Getwalk_blend)))) false true)
  (Variables|Player|Motionstate|Setvisual_lean (Math|Interpolation|FInterpTo (Variables|Player|Motionstate|Getvisual_lean) (* (/ (.X (Math|Vector|BreakVector _returnvalue)) (Math|Float|Max(Float) (Variables|Player|Getmove_speed) 1.0)) (Variables|Player|Getwalk_lean_degrees)) _returnvalue_2 14.0))
  (Transformation|SetRelativeRotation _player_visual (Math|Rotator|MakeRotator 0.0 (Variables|Player|Motionstate|Getvisual_lean) 0.0) false true)
  (Rendering|SetTranslucentSortPriority _player_visual _returnvalue_13)
  (Rendering|SetVisibility _walk_right_foot (Variables|Player|Motionstate|Getis_moving) false)
  (Rendering|SetTranslucentSortPriority _walk_right_foot _returnvalue_13)
  (Sprite|SetSpriteColor _walk_right_foot _spritecolor)
  (Transformation|SetRelativeLocation _walk_right_foot (Math|Vector|MakeVector (* (* (Math|Trig|Sin(Radians) (* (Math|Conversions|ToFloat(Integer) (Variables|Player|Motionstate|Getcurrent_frame_index)) 0.7853981633974483)) -1.0) (Math|Float|SelectFloat 1.25 0.25 (>= (Variables|Player|Motionstate|Getfacing_direction) 2))) 0.0 (* (Math|Float|Max(Float) 0.0 (* (Math|Trig|Sin(Radians) (* (Math|Conversions|ToFloat(Integer) (Variables|Player|Motionstate|Getcurrent_frame_index)) 0.7853981633974483)) -1.0)) 1.25)) false true)
  (Rendering|SetVisibility _walk_left_foot (Variables|Player|Motionstate|Getis_moving) false)
  (Rendering|SetTranslucentSortPriority _walk_left_foot _returnvalue_13)
  (Sprite|SetSpriteColor _walk_left_foot _spritecolor)
  (Transformation|SetRelativeLocation _walk_left_foot (Math|Vector|MakeVector (* (Math|Trig|Sin(Radians) (* (Math|Conversions|ToFloat(Integer) (Variables|Player|Motionstate|Getcurrent_frame_index)) 0.7853981633974483)) (Math|Float|SelectFloat 1.25 0.25 (>= (Variables|Player|Motionstate|Getfacing_direction) 2))) 0.01 (* (Math|Float|Max(Float) 0.0 (Math|Trig|Sin(Radians) (* (Math|Conversions|ToFloat(Integer) (Variables|Player|Motionstate|Getcurrent_frame_index)) 0.7853981633974483))) 1.25)) false true)
  (Rendering|SetVisibility _walk_body (Variables|Player|Motionstate|Getis_moving) false)
  (Rendering|SetTranslucentSortPriority _walk_body _returnvalue_13)
  (Sprite|SetSpriteColor _walk_body _spritecolor)
  (Transformation|SetRelativeLocation _walk_body (Math|Vector|MakeVector (* (Math|Trig|Sin(Radians) (* (Math|Conversions|ToFloat(Integer) (Variables|Player|Motionstate|Getcurrent_frame_index)) 0.7853981633974483)) 0.0) 0.02 (- (* (Math|Trig|Cos(Radians) (* (* (Math|Conversions|ToFloat(Integer) (Variables|Player|Motionstate|Getcurrent_frame_index)) 0.7853981633974483) 2.0)) 0.55) 0.55)) false true)
  (Rendering|SetVisibility _walk_head (Variables|Player|Motionstate|Getis_moving) false)
  (Rendering|SetTranslucentSortPriority _walk_head _returnvalue_13)
  (Sprite|SetSpriteColor _walk_head _spritecolor)
  (Transformation|SetRelativeLocation _walk_head (Math|Vector|MakeVector (* (Math|Trig|Sin(Radians) (* (Math|Conversions|ToFloat(Integer) (Variables|Player|Motionstate|Getcurrent_frame_index)) 0.7853981633974483)) 0.15) 0.03 (- (* (Math|Trig|Cos(Radians) (- (* (* (Math|Conversions|ToFloat(Integer) (Variables|Player|Motionstate|Getcurrent_frame_index)) 0.7853981633974483) 2.0) 0.4)) 0.35) 0.35)) false true))