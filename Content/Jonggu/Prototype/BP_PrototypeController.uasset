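; Prototype player controller that forwards local mouse and keyboard input to BP_PrototypeManager, ticking even while the game is paused.
; BeginPlay sets Game and UI input mode for the local player.
; Each tick maps the cursor into a letterboxed 1280x720 virtual canvas, using -1 when outside, and updates the manager's pointer.
; Key presses then trigger one action by priority: pause toggle, interact, or click at that pointer.
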(event EventBeginPlay
  (Class|Actor|SetTickablewhenPaused true)
  (Actor|Tick|SetActorTickEnabled true)
  (if (Pawn|IsLocalController)
    (Input|SetInputModeGameandUI (Game|GetPlayerController 0) 0 "DoNotLock" false true)))

(event EventTick
  (params (DeltaSeconds :type Float%20%28single-precision%29))
  (bind (_locationx _locationy _returnvalue) (Game|Player|GetMousePosition))
  (bind (_sizex _sizey) (HUD|GetViewportSize))
  (bind _returnvalue_2 (Math|Conversions|ToFloat(Integer) _sizex))
  (bind _returnvalue_3 (Math|Conversions|ToFloat(Integer) _sizey))
  (bind _returnvalue_4 (/ _returnvalue_2 1.28e+03))
  (bind _returnvalue_5 (/ _returnvalue_3 7.2e+02))
  (bind _returnvalue_6 (Math|Float|Min(Float) _returnvalue_4 _returnvalue_5))
  (bind _returnvalue_7 (* 1.28e+03 _returnvalue_6))
  (bind _returnvalue_8 (* 7.2e+02 _returnvalue_6))
  (bind _returnvalue_9 (- _returnvalue_2 _returnvalue_7))
  (bind _returnvalue_10 (- _returnvalue_3 _returnvalue_8))
  (bind _returnvalue_11 (* _returnvalue_9 0.5))
  (bind _returnvalue_12 (* _returnvalue_10 0.5))
  (bind _returnvalue_13 (- _locationx _returnvalue_11))
  (bind _returnvalue_14 (- _locationy _returnvalue_12))
  (bind _returnvalue_15 (/ _returnvalue_13 _returnvalue_6))
  (bind _returnvalue_16 (/ _returnvalue_14 _returnvalue_6))
  (if (Pawn|IsLocalController)
    (bind _returnvalue_17 (Actor|GetActorOfClass "/Game/Jonggu/Prototype/BP_PrototypeManager.BP_PrototypeManager_C"))
    (if (Utilities|IsValid _returnvalue_17)
      (Variables|Default|Setpointer_x -1.0)
      (Variables|Default|Setpointer_y -1.0)
      (if (and _returnvalue (and (> _sizex 0) (> _sizey 0)))
        (if (and (and (>= _returnvalue_15 0.0) (< _returnvalue_15 1.28e+03)) (and (>= _returnvalue_16 0.0) (< _returnvalue_16 7.2e+02)))
          (Variables|Default|Setpointer_x _returnvalue_15)
          (Variables|Default|Setpointer_y _returnvalue_16)))
      (Default|UpdatePointer _returnvalue_17 (Variables|Default|Getpointer_x) (Variables|Default|Getpointer_y) (Game|Player|IsInputKeyDown "LeftMouseButton"))
      (if (or (Game|Player|WasInputKeyJustPressed "Escape") (Game|Player|WasInputKeyJustPressed "F10"))
        (Default|PauseToggle _returnvalue_17)
        (elif (Game|Player|WasInputKeyJustPressed "E")
          (Default|Interact _returnvalue_17)
          (elif (Game|Player|WasInputKeyJustPressed "LeftMouseButton")
            (Default|Click _returnvalue_17 (Variables|Default|Getpointer_x) (Variables|Default|Getpointer_y))))))))

(fn ConstructionScript)